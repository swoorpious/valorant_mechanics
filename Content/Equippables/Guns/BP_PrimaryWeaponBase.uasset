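; Base Blueprint for primary guns that draws a Niagara bullet tracer whenever a shot is reported.
; The beam runs from the muzzle bone, adjusted through ViewModelWPO, to the impact point or a far point along the camera's aim on a miss.
; A timeline scaled by distance keeps travel speed constant, sliding a segment capped at MaxBeamLength along the path, then destroying it.
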(event `self.ReceiveBeginPlay`
  (bind _returnvalue_location (`KismetMathLibrary.BreakTransform` (`SkinnedMeshComponent.GetBoneTransform` (`self.weaponMesh`) "MuzzlePoint" "RTS_Actor")))
  (bind _asval_player_controller (cast `Val_PlayerController` (`GameplayStatics.GetPlayerController` 0)))
  (set `self.Player Controller` _asval_player_controller)
  (set `self.Tracer Start Offset` _returnvalue_location))

(event `self.receiveOnWeaponEquipped`)

(event `self.receiveOnBulletShot`
  (params (hitSomething :type Boolean) (HitResult :type "HitResult Structure"))
  (bind _r (`self.R`))
  (bind _weaponmesh (`self.weaponMesh`))
  (bind _returnvalue_location (`KismetMathLibrary.BreakTransform` (`SkinnedMeshComponent.GetBoneTransform` _weaponmesh "MuzzlePoint" "RTS_World")))
  (bind _charactermeshcamera (`Val_Character.characterMeshCamera` (`self._ownerCharacter_`)))
  (bind _returnvalue (`self._viewModelWPO` _returnvalue_location))
  (bind _returnvalue_2 (select `bool` hitSomething :`false` (+ (* (`SceneComponent.GetForwardVector` _charactermeshcamera) 10000.0) (`SceneComponent.K2_GetComponentLocation` _charactermeshcamera)) :`true` (`.ImpactPoint` (`GameplayStatics.BreakHitResult` HitResult))))
  (bind _returnvalue_3 (`KismetMathLibrary.Vector_Distance` _returnvalue _returnvalue_2))
  (`/Engine/EditorBlueprintResources/StandardMacros.IsValid` _weaponmesh
    (:`Is Valid`
      (bind _returnvalue_4 (`NiagaraFunctionLibrary.SpawnSystemAtLocation` "/Game/VFX/NS_BulletTracer.NS_BulletTracer" _returnvalue))
      (`TimelineComponent.SetPlayRate` (`self.Tracer Timeline`) (/ 10000.0 _returnvalue_3))
      (bind (_direction _alpha) (`Timeline|Tracer Timeline` :!via `PlayFromStart` :!label _label)
        (:`Update`
          (`/Engine/EditorBlueprintResources/StandardMacros.IsValid` _returnvalue_4
            (:`Is Valid`
              (if (>= _returnvalue_3 0.0)
                (set `self.R` (/ (`self.Max Beam Length`) _returnvalue_3))
                (bind _returnvalue_5 (* (+ _r 1.0) _alpha))
                (`FXSystemComponent.SetVectorParameter` _returnvalue_4 "Beam Start" (`KismetMathLibrary.VLerp` _returnvalue _returnvalue_2 (`KismetMathLibrary.FClamp` (- _returnvalue_5 _r))))
                (`FXSystemComponent.SetVectorParameter` _returnvalue_4 "Beam End" (`KismetMathLibrary.VLerp` _returnvalue _returnvalue_2 (`KismetMathLibrary.FClamp` _returnvalue_5)))))
            (:`Is Not Valid`
              (goto _label :!via `Stop`))))
        (:`Finished`
          (`ActorComponent.K2_DestroyComponent` _returnvalue_4))))))

(fn `UserConstructionScript`)